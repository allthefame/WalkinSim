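; Actor component that adds wall jumping to BP_ThirdPersonCharacter through the character's prep and action events.
; On prep, a falling character traces forward for a BP_InteractableWall and, if allowed, has its velocity damped toward zero.
; Attempts are limited per wall, resetting on a different wall or after a cooldown triggered once they run out.
; The action event launches the character with forward-axis force plus upward thrust, then rotates its yaw, without rechecking those conditions.
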(event `self.ReceiveBeginPlay`
  ; Wall Jumping
  (bind _asbp_third_person_character (cast `/Game/ThirdPerson/Blueprints/BP_ThirdPersonCharacter` (`self.GetOwner`)))
  (set `self.CharRef` _asbp_third_person_character)
  (`|ExecutionSequence`
    (:`then_0`
      ;;[0.8531 0 0 0.5] Setup
      (add `/Game/ThirdPerson/Blueprints/BP_ThirdPersonCharacter.WallJumpPrep` (`self.CharRef`) (delegate `WallJumpPrepEvent`)))
    (:`then_1`
      ;;[0 0.3916 0.7781 0.5] Fuctionality
      (add `/Game/ThirdPerson/Blueprints/BP_ThirdPersonCharacter.WallJumpAction` (`self.CharRef`) (delegate `WallJumpActionEvent`)))))

(event `WallJumpPrepEvent`
  (params (Movement :type "CharacterMovementComponent Object Reference") (CapsuleComponent :type "CapsuleComponent Object Reference"))
  ; Wall Jumping
  ;;[0.8531 0 0 0.5] Setup
  (`self.WallJumpSetter` Movement CapsuleComponent))

(event `JumpCooldownEvent`
  ; Wall Jumping
  ;;[0 0.4781 0.1221 0.5] Cooldown
  (`|ExecutionSequence`
    (:`then_0`
      (set `self.IsCountdownActive` true))
    (:`then_1`
      (`KismetSystemLibrary.Delay` (`self.JumpCooldown`))
      (set `self.IsCountdownActive` false)
      (set `self.#OfCurrentJumps` (`self.#OfMaxJumps`)))))

(event `WallJumpActionEvent`
  ; Wall Jumping
  ;;[0 0.3916 0.7781 0.5] Fuctionality
  (`self.ExecuteWallJump` (`self.CharRef`)))

(fn `ChangeWallboundVelocity`
  (params (Movement :type "CharacterMovementComponent Object Reference"))
  (set `MovementComponent.Velocity` (`KismetMathLibrary.VInterpTo` (`MovementComponent.Velocity` Movement) (0.0 0.0 0.0) (`GameplayStatics.GetWorldDeltaSeconds`) (`self.SpeedDecrease`)) Movement))

(fn `ExecuteWallJump`
  (params (CharRef :type "/Game/ThirdPerson/Blueprints/BP_ThirdPersonCharacter Object Reference"))
  (bind (_returnvalue_roll _returnvalue_pitch _returnvalue_yaw) (`KismetMathLibrary.BreakRotator` (`Actor.K2_GetActorRotation` CharRef)))
  (`Character.LaunchCharacter` CharRef (+ (* (`Actor.GetActorForwardVector` CharRef) (`self.WallJumpForce`)) (`KismetMathLibrary.MakeVector` 0.0 0.0 (`self.UpwardThrust`))) true true)
  (`Actor.K2_SetActorRotation` CharRef (`KismetMathLibrary.MakeRotator` _returnvalue_roll _returnvalue_pitch (+ _returnvalue_yaw (`self.FlipCharacter`))) false))

(fn `JumpAttemptsOnThisWall`
  (returns (Result :type Boolean))
  (bind _returnvalue (`KismetSystemLibrary.GetObjectName` (`self.CheckedWall`)))
  ; Is it the same wall?
  (if (`KismetStringLibrary.EqualEqual_StrStr` _returnvalue (`self.PreviousWall`))
    ; Is jump cooldown timer not active? (/paused?)
    (if (not (`self.IsCountdownActive`))
      ; Have enough wall jumps on this wall?
      (if (> (`self.#OfCurrentJumps`) 0)
        ; If Yes
        (set `self.#OfCurrentJumps` (- (`self.#OfCurrentJumps`) 1))
        (bind _output_get (set `self.CanJumpOnThisWall?` true))
        (return _output_get)
        (else
          ; If No
          (`self.JumpCooldownEvent`)
          (return false)))
      (else
        (return false)))
    (else
      ; Reset Wall Jump Chances
      (set `self.PreviousWall` _returnvalue)
      (set `self.#OfCurrentJumps` (- (`self.#OfMaxJumps`) 1))
      (bind _output_get_2 (set `self.CanJumpOnThisWall?` true))
      (return _output_get_2))))

(fn `WallJumpConditionsChecker`
  (params (Movement :type "CharacterMovementComponent Object Reference") (CapsuleComponent :type "CapsuleComponent Object Reference"))
  (returns (Result :type Boolean) (Move :type "CharacterMovementComponent Object Reference"))
  (if (`NavMovementInterface.IsFalling` Movement)
    ;[0.001655 1 0 0.5] Wall Checker
    (bind _result (`self.WallSearcherBuilder` CapsuleComponent))
    (if _result
      (bind _result_2 (`self.JumpAttemptsOnThisWall`))
      (return _result_2 Movement)
      (else
        _)))
  (bind _output_get (set `self.CanWallJump?` false))
  (return _output_get null))

(fn `WallJumpSetter`
  (params (Movement :type "CharacterMovementComponent Object Reference") (CapsuleComponent :type "CapsuleComponent Object Reference"))
  (bind (_result _move) (`self.WallJumpConditionsChecker` Movement CapsuleComponent))
  (bind _output_get (set `self.CanWallJump?` _result))
  (if _output_get
    (`self.ChangeWallboundVelocity` _move)))

(fn `WallSearcherBuilder`
  (params (CapsuleComponent :type "CapsuleComponent Object Reference"))
  (returns (Result :type Boolean))
  (bind _returnvalue (`SceneComponent.K2_GetComponentLocation` CapsuleComponent))
  ; Wall Searcher
  (bind (_outhit _returnvalue_2) (`KismetSystemLibrary.LineTraceSingleForObjects` _returnvalue (+ _returnvalue (* (`SceneComponent.GetForwardVector` CapsuleComponent) (`self.WallCheckerDistance`))) (`self.Object Types - Walls`)))
  (if _returnvalue_2
    (bind _result (`self.WallTypeChecker` (`.HitActor` (`GameplayStatics.BreakHitResult` _outhit))))
    (return _result)))

(fn `WallTypeChecker`
  (params (CheckedWall :type "Actor Object Reference"))
  (returns (Result :type Boolean))
  (set `self.CheckedWall` CheckedWall)
  (return (`KismetMathLibrary.ClassIsChildOf` (`GameplayStatics.GetObjectClass` CheckedWall) "/Game/Blueprints/Items/BP_InteractableWall.BP_InteractableWall_C")))