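; Inventory component for BP_ThirdPersonCharacter that finds, adds and removes items in HUD slots.
; It keeps no item list of its own, reading slot state directly from the SlotArray of the character's MainHUDWidget.
; Adds and removals fire OnInventoryUpdatedAtSlot, which the component itself binds to push changes into the widget via SlotUpdated.
; Four debug keys remove items from the first four slots.
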(event Custom|UpdateInventory
  (params (Index :type Integer) (Item :type BP%20Inventory%20Item%20Object%20Reference) (EmptySlot :type Boolean))
  (Default|SlotUpdated (Variables|/Game/ThirdPerson/Blueprints/BP_ThirdPersonCharacter.BP_ThirdPersonCharacter_C|GetMainHUDWidget (Variables|Default|GetCharRef)) Index Item EmptySlot))

(event EventBeginPlay
  (bind _asbp_third_person_character (Utilities|Casting|CastToBP_ThirdPersonCharacter (Components|GetOwner)))
  (Variables|Default|SetCharRef _asbp_third_person_character)
  (EventDispatchers|BindEventtoOnInventoryUpdatedatSlot (delegate Custom|UpdateInventory)))

(event Input|KeyboardEvents|DebugKey1
  (params (Key :type Key%20Structure :default "None") (ActionValue :type Input%20Action%20Value%20Structure))
  (:Pressed
    (CallFunction|RemoveItematIndex)))

(event Input|KeyboardEvents|DebugKey2
  (params (Key :type Key%20Structure :default "None") (ActionValue :type Input%20Action%20Value%20Structure))
  (:Pressed
    (CallFunction|RemoveItematIndex 1)))

(event Input|KeyboardEvents|DebugKey3
  (params (Key :type Key%20Structure :default "None") (ActionValue :type Input%20Action%20Value%20Structure))
  (:Pressed
    (CallFunction|RemoveItematIndex 2)))

(event Input|KeyboardEvents|DebugKey4
  (params (Key :type Key%20Structure :default "None") (ActionValue :type Input%20Action%20Value%20Structure))
  (:Pressed
    (CallFunction|RemoveItematIndex 3)))

(fn CanAddItemtoInventory
  (params (ItemToAdd :type BP%20Inventory%20Item%20Object%20Reference))
  (for (_array_element _array_index) (Variables|/Game/Blueprints/UI/HUD/WBP_MainHUD.WBP_MainHUD_C|GetSlotArray (Variables|/Game/ThirdPerson/Blueprints/BP_ThirdPersonCharacter.BP_ThirdPersonCharacter_C|GetMainHUDWidget (Variables|Default|GetCharRef)))
    (if (Variables|/Game/Blueprints/UI/Inventory/WBP_ItemSlot.WBP_ItemSlot_C|GetEmpty%20Slot _array_element)
      (return _array_index ItemToAdd true)))
  (return 0 0 false))

(fn AddItemtoInventory
  (params (Index :type Integer) (Item :type BP%20Inventory%20Item%20Object%20Reference))
  (Default|CallOnInventoryUpdatedatSlot Index Item false))

(fn FindItem
  (params (ItemToFind :type BP%20Inventory%20Item%20Object%20Reference))
  (for (_array_element _array_index) (Variables|/Game/Blueprints/UI/HUD/WBP_MainHUD.WBP_MainHUD_C|GetSlotArray (Variables|/Game/ThirdPerson/Blueprints/BP_ThirdPersonCharacter.BP_ThirdPersonCharacter_C|GetMainHUDWidget (Variables|Default|GetCharRef)))
    (if (== (Variables|/Game/Blueprints/UI/Inventory/WBP_ItemSlot.WBP_ItemSlot_C|GetItem _array_element) ItemToFind)
      (return _array_index true)))
  (return 0 false))

(fn RemoveItem
  (params (ItemToRemove :type BP%20Inventory%20Item%20Object%20Reference))
  (bind (_index _found) (CallFunction|FindItem ItemToRemove))
  (if _found
    (Default|CallOnInventoryUpdatedatSlot _index 0 true)
    (else
      (Development|PrintString "Item to Remove didn't exist"))))

(fn FindItematIndex
  (params (Index :type Integer))
  (bind _charref (Variables|Default|GetCharRef))
  (bind _mainhudwidget (Variables|/Game/ThirdPerson/Blueprints/BP_ThirdPersonCharacter.BP_ThirdPersonCharacter_C|GetMainHUDWidget _charref))
  (bind _slotarray (Variables|/Game/Blueprints/UI/HUD/WBP_MainHUD.WBP_MainHUD_C|GetSlotArray _mainhudwidget))
  (bind _output (Utilities|Array|Get(acopy) _slotarray Index))
  (Utilities|IsValid _output
    (:Is%20Valid
      (return (Variables|/Game/Blueprints/UI/Inventory/WBP_ItemSlot.WBP_ItemSlot_C|GetItem _output) true))
    (:Is%20Not%20Valid
      (return 0 false))))

(fn RemoveItematIndex
  (params (Index :type Integer))
  (bind _found (CallFunction|FindItematIndex Index))
  (if _found
    (Default|CallOnInventoryUpdatedatSlot Index 0 true)))