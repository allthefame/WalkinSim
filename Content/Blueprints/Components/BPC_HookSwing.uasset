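; Character component that runs a grappling hook swing, driven by events bound on BP_ThirdPersonCharacter.
; Prep takes the first BP_LatchableSurface in hookable range, faces it along Y, spawns the hook and constrains the capsule to it via a spawned PhysicsConstraintActor.
; Travel events lerp the hook to target; swinging disables movement mode and gravity, with A/D setting Y-axis cable force.
; Cleanup restores falling and destroys hook and constraint.
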(event `self.ReceiveBeginPlay`
  ; Hook Swing
  (bind _asbp_third_person_character (cast `/Game/ThirdPerson/Blueprints/BP_ThirdPersonCharacter` (`self.GetOwner`)))
  (set `self.CharRef` _asbp_third_person_character)
  (`|ExecutionSequence`
    (:`then_0`
      ;;[0.5823 0 0 0.5] Setup
      (add `/Game/ThirdPerson/Blueprints/BP_ThirdPersonCharacter.HookSwingPrep` (`self.CharRef`) (delegate `OnHookSwingPrep`))
      (add `/Game/ThirdPerson/Blueprints/BP_ThirdPersonCharacter.HookTravelManager` (`self.CharRef`) (delegate `OnHookTravelManagement`)))
    (:`then_1`
      ;;[0 0.2919 0.7906 0.5] Functionality
      (add `/Game/ThirdPerson/Blueprints/BP_ThirdPersonCharacter.HookSwingAction` (`self.CharRef`) (delegate `OnHookSwingAction`)))
    (:`then_2`
      ;;[0 0.649 0.2057 0.5] Deconstruction
      (add `/Game/ThirdPerson/Blueprints/BP_ThirdPersonCharacter.HookSwingCleanup` (`self.CharRef`) (delegate `OnHookSwingCleanup`)))))

(event `OnHookSwingPrep`
  ; Hook Swing
  ;;[0.5823 0 0 0.5] Setup
  (`self.GrapplingHookSetup`))

(event `OnHookTravelManagement`
  (params (CableFlyTime :type "Float (double-precision)"))
  ; Hook Swing
  ;;[0.5823 0 0 0.5] Setup
  (`self.SendCableToLocation` CableFlyTime))

(event `Key|A`
  (params (Key :type "Key Structure"))
  (bind _grapplinghook (`self.GrapplingHook`))
  ; Hook Swing
  ;; Swing Movement
  (:`Pressed`
    (`/Engine/EditorBlueprintResources/StandardMacros.IsValid` _grapplinghook
      (:`Is Valid`
        (`self.CableForce-` (`/Game/Blueprints/Items/BP_GrapplingHook.Cable` _grapplinghook))))))

(event `Key|D`
  (params (Key :type "Key Structure"))
  (bind _grapplinghook (`self.GrapplingHook`))
  ; Hook Swing
  ;; Swing Movement
  (:`Pressed`
    (`/Engine/EditorBlueprintResources/StandardMacros.IsValid` _grapplinghook
      (:`Is Valid`
        (`self.CableForce+` (`/Game/Blueprints/Items/BP_GrapplingHook.Cable` _grapplinghook))))))

(event `OnHookSwingAction`
  ; Hook Swing
  ;;[0 0.2919 0.7906 0.5] Functionality
  (`self.HookSwingState`))

(event `OnHookSwingCleanup`
  ; Hook Swing
  ;;[0 0.649 0.2057 0.5] Deconstruction
  (`self.CleanupManager`))

(event `CleanupManager`
  ; Hook Swing
  ;; Cleanup
  (`/Game/ThirdPerson/Blueprints/BP_ThirdPersonCharacter.StopHook` (`self.CharRef`))
  (`self.StopGrappling`)
  (`self.RemoveGrappling`))

(fn `AttachToLatchableSurface`
  (bind _cable (`/Game/Blueprints/Items/BP_GrapplingHook.Cable` (`self.GrapplingHook`)))
  (`/Game/ThirdPerson/Blueprints/BP_ThirdPersonCharacter.MoveHook` (`self.CharRef`))
  (if (not (`CableComponent.bAttachStart` _cable))
    (set `CableComponent.bAttachStart` true _cable)))

(fn `CableForce+`
  (params (InputPin :type "CableComponent Object Reference"))
  (set `CableComponent.CableForce` (`KismetMathLibrary.MakeVector` 0.0 (`self.CableForce`)) InputPin)
  (`KismetSystemLibrary.PrintString` "Right"))

(fn `CableForce-`
  (params (HookCable :type "CableComponent Object Reference"))
  (set `CableComponent.CableForce` (`KismetMathLibrary.MakeVector` 0.0 (* (`self.CableForce`) -1.0)) HookCable)
  (`KismetSystemLibrary.PrintString` "Left"))

(fn `CheckForLatchableSurfaces`
  (params (HookableRange :type "SphereComponent Object Reference"))
  (returns (`Latchable Surface` :type "/Game/Blueprints/Items/BP_LatchableSurface Object Reference"))
  (bind _asbp_latchable_surface (cast `/Game/Blueprints/Items/BP_LatchableSurface` (`|GetArrayItem` (`PrimitiveComponent.GetOverlappingActors` HookableRange "/Game/Blueprints/Items/BP_LatchableSurface.BP_LatchableSurface_C"))))
  (bind _output_get (set `self.LatchableObject` _asbp_latchable_surface))
  (return _output_get))

(fn `FaceLatchableObject`
  (bind _charref (`self.CharRef`))
  (bind (_returnvalue_x _returnvalue_y) (`KismetMathLibrary.BreakVector` (`Actor.K2_GetActorLocation` _charref)))
  (bind (_returnvalue_x_2 _returnvalue_y_2) (`KismetMathLibrary.BreakVector` (`Actor.K2_GetActorLocation` (`self.LatchableObject`))))
  (if (< _returnvalue_y_2 _returnvalue_y)
    (`Actor.K2_SetActorRotation` _charref (`self.FacingLeft`) false)
    (else
      (`Actor.K2_SetActorRotation` _charref (`self.FacingRight`) false))))

(fn `GrapplingHookSetup`
  (if (not (`self.IsGrappling`))
    (bind _latchable_surface (`self.CheckForLatchableSurfaces` (`/Game/ThirdPerson/Blueprints/BP_ThirdPersonCharacter.Hookable Range` (`self.CharRef`))))
    (`/Engine/EditorBlueprintResources/StandardMacros.IsValid` _latchable_surface
      (:`Is Valid`
        (`self.RevealLatchableObject`)
        (`self.HookCheck`)
        (`self.FaceLatchableObject`)
        (`self.HookCableCrafter`)
        (`self.AttachToLatchableSurface`)
        (`self.HookConstraintSetter`)
        (set `self.IsGrappling` true))
      (:`Is Not Valid`
        (set `self.IsGrappling` false)))))

(fn `HookCableCrafter`
  (bind _returnvalue (`|SpawnActorFromClass` "/Game/Blueprints/Items/BP_GrapplingHook.BP_GrapplingHook_C" (`Actor.GetTransform` (`self.CharRef`)) "Undefined" "MultiplyWithRoot" null null))
  (set `self.GrapplingHook` _returnvalue))

(fn `HookCheck`
  (if (not (`KismetSystemLibrary.IsValid` (`self.GrapplingHook`)))
    (return)))

(fn `HookConstraintSetter`
  (bind _returnvalue (`|SpawnActorFromClass` "/Script/Engine.PhysicsConstraintActor" (`KismetMathLibrary.TLerp` (`Actor.GetTransform` (`self.CharRef`)) (`Actor.GetTransform` (`self.LatchableObject`)) (`self.ConstraintTether`)) "Undefined" "MultiplyWithRoot" null null))
  (set `self.HookRestraint` _returnvalue)
  (`self.SetConstraintEnds`))

(fn `HookSwingState`
  (if (and (`self.IsGrappling`) (`KismetSystemLibrary.IsValid` (`self.GrapplingHook`)))
    (`CharacterMovementComponent.SetMovementMode` (`Character.CharacterMovement` (`self.CharRef`)) "MOVE_None" 0)
    (`PrimitiveComponent.SetEnableGravity` (`Character.CapsuleComponent` (`self.CharRef`)) false)))

(fn `RemoveGrappling`
  (bind _hookrestraint (`self.HookRestraint`))
  (bind _grapplinghook (`self.GrapplingHook`))
  (`/Engine/EditorBlueprintResources/StandardMacros.IsValid` _hookrestraint
    (:`Is Valid`
      (`Actor.K2_DestroyActor` _hookrestraint))
    (:`Is Not Valid`
      _))
  (`/Engine/EditorBlueprintResources/StandardMacros.IsValid` _grapplinghook
    (:`Is Valid`
      (`Actor.K2_DestroyActor` _grapplinghook))))

(fn `RevealLatchableObject`
  (`KismetSystemLibrary.DrawDebugPoint` (`Actor.K2_GetActorLocation` (`self.LatchableObject`)) 100.0 (struct :`G` 0.757759 :`B` 1.0 :`A` 1.0) 0.3))

(fn `SendCableToLocation`
  (params (CableFlyTime :type "Float (double-precision)"))
  (bind _grapplinghook (`self.GrapplingHook`))
  (if (`KismetSystemLibrary.IsValid` (`self.GrapplingHook`))
    (`Actor.K2_SetActorLocation` _grapplinghook (`KismetMathLibrary.VLerp` (`Actor.K2_GetActorLocation` _grapplinghook) (`Actor.K2_GetActorLocation` (`self.LatchableObject`)) CableFlyTime) false false)))

(fn `SetConstraintEnds`
  (bind _sphere (`/Game/Blueprints/Items/BP_LatchableSurface.Sphere` (`self.LatchableObject`)))
  (bind _capsulecomponent (`Character.CapsuleComponent` (`self.CharRef`)))
  (`PhysicsConstraintComponent.SetConstrainedComponents` (`PhysicsConstraintActor.ConstraintComp` (`self.HookRestraint`)) _sphere (`KismetStringLibrary.Conv_StringToName` (`KismetSystemLibrary.GetObjectName` _sphere)) _capsulecomponent (`KismetStringLibrary.Conv_StringToName` (`KismetSystemLibrary.GetObjectName` _capsulecomponent))))

(fn `StopGrappling`
  (if (`self.IsGrappling`)
    (set `self.IsGrappling` false)
    (`CharacterMovementComponent.SetMovementMode` (`Character.CharacterMovement` (`self.CharRef`)) "MOVE_Falling" 0)))