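; BP_Hero is a player-controlled test hero with Enhanced Input movement.
; On BeginPlay it casts its controller to PlayerController and calls AddMappingContext on the Enhanced Input subsystem, with no context asset shown.
; IA_TestMove stores its value in Directionality and feeds X and Y into movement input along fixed world axes, independent of camera or control rotation.
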(event `self.ReceiveBeginPlay`
  ; Setting Up Player Controls
  (bind _asplayer_controller (cast `PlayerController` (`self.GetController`)))
  (`EnhancedInputSubsystemInterface.AddMappingContext` (pcsubsystem `EnhancedInputLocalPlayerSubsystem` _asplayer_controller) null 0 (struct)))

(event `EnhancedInput|/Game/Inputs/TestInputs/Actions/IA_TestMove`
  (params (ActionValue :type "Vector2D Structure") (ElapsedSeconds :type "Float (double-precision)") (TriggeredSeconds :type "Float (double-precision)") (InputAction :type "InputAction Object Reference" :default "/Game/Inputs/TestInputs/Actions/IA_TestMove.IA_TestMove"))
  (bind (_x _y) (`KismetMathLibrary.BreakVector2D` ActionValue))
  ; Movement
  (:`Triggered`
    (set `self.Directionality` ActionValue)
    (`self.AddMovementInput` (1.0 0.0 0.0) _x)
    (`self.AddMovementInput` (0.0 1.0 0.0) _y)))

(fn `UserConstructionScript`
  (`parent.UserConstructionScript`))