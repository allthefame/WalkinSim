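; Base Blueprint for an interactable door that opens through a Level Sequence and can be linked to a key item.
; On BeginPlay it caches the inventory item of its assigned world key object, exposed through GetDoorKey.
; Interaction disables door collision and plays the open sequence on a newly created sequence player, with no key check in this graph.
; Its own GetInventoryItem returns nothing.
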(event `self.ReceiveBeginPlay`
  (bind _worldkeyobj (`self.WorldKeyObj`))
  (`/Engine/EditorBlueprintResources/StandardMacros.IsValid` _worldkeyobj
    (:`Is Valid`
      (bind _item (`/Game/Blueprints/Items/BP_PickupBase.GetInventoryItem` _worldkeyobj))
      (set `self.WorldKeyItem` _item))))

(event `/Game/Blueprints/Interfaces/BPI_InteractableObject.WorldObjectInteract`
  (`PrimitiveComponent.SetCollisionEnabled` (`self.Door`) "NoCollision")
  (bind _outactor (`LevelSequencePlayer.CreateLevelSequencePlayer` (`self.DoorOpenSequence`)))
  (`MovieSceneSequencePlayer.Play` (`LevelSequenceActor.SequencePlayer` _outactor)))

(fn `GetDoorKey`
  (returns (Key :type "/Game/Blueprints/Inventory/BP_InventoryItem Object Reference"))
  (return (`self.WorldKeyItem`)))

(fn `GetInventoryItem`
  (returns (Item :type "/Game/Blueprints/Inventory/BP_InventoryItem Object Reference"))
  (return null))

(fn `UserConstructionScript`)